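; Population counter actor that shows a live player count on a TextRender.
; A self-restarting delay timer refreshes the count from either the GameMode's player total or a multi sphere trace, chosen by a flag.
; The trace counts hits on the "b_ch_head" bone rather than casting, so it also works with custom game modes.
; The construction script applies text color and a sample count for preview.
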(event Custom|StartTimer
  ;[1 1 1] Timer
  (Utilities|FlowControl|Delay (Variables|Default|GetCheckTimer))
  (Utilities|FlowControl|Sequence
    (:then_0
      (if (Variables|Default|GetBase%20on%20player%20count%20%28simplified%29)
        ;[1 1 1] Get how many players are in server//Set population
        (bind _asgame_mode (Utilities|Casting|CastToGameMode (Game|GetGameMode)))
        (bind _returnvalue (Class|GameModeBase|GetNumPlayers _asgame_mode))
        (Rendering|Components|TextRender|SetText (Variables|Default|GetTextRender) (Utilities|Text|ToText(Integer) _returnvalue))
        (else
          ;[1 1 1] Scan For Players//Set Player Count
          (Variables|Default|SetPlayerCount 0)
          (bind _outhits (Collision|MultiSphereTraceForObjects (Transformation|GetActorLocation) (* (Math|Vector|GetForwardVector (Transformation|GetActorRotation)) 5e+03) (Variables|Default|GetDistance%20To%20Check%20For%20Players) (Variables|Default|GetTypeToSearchFor) false 0 (Variables|Default|GetDebug%20Draw)))
          (for _array_element _outhits
            (if (Utilities|Name|Equal(Name) (.HitBoneName (Collision|BreakHitResult _array_element)) "b_ch_head")
              (Variables|Default|SetPlayerCount (+ (Variables|Default|GetPlayerCount) 1))))
          ;[1 1 1] Set Population Text
          (Rendering|Components|TextRender|SetText (Variables|Default|GetTextRender) (Utilities|Text|ToText(Integer) (Variables|Default|GetPlayerCount))))))
    (:then_1
      (CallFunction|StartTimer))))

(event EventBeginPlay
  ;[1 1 1] Start Timer (when game starts)
  (CallFunction|StartTimer))

(fn ConstructionScript
  (bind _textrender (Variables|Default|GetTextRender))
  (Rendering|Components|TextRender|SetTextRenderColor _textrender (Variables|Default|GetText%20Color))
  (Rendering|Components|TextRender|SetText _textrender (Utilities|Text|ToText(Integer) (Variables|Default|GetSample%20Player%20Count))))